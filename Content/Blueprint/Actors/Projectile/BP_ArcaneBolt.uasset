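; BP_ArcaneBolt is a projectile that deals area damage around itself through the Gameplay Ability System.
; Its ApplyRangeDamage event passes the hit actor to ApplyExplodeDamage, which sphere-traces at the bolt's location, ignoring that actor and the owner.
; Each non-friendly actor found is recorded in DamagedActor, so it receives the DamageSpecHandle gameplay effect only once.
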(event EventBeginPlay)

(event EventApplyRangeDamage
  (params (HitActor :type Actor%20Object%20Reference))
  (CallFunction|ApplyExplodeDamage HitActor))

(fn ConstructionScript)

(fn ApplyExplodeDamage
  (params ([0] :type Actor%20Object%20Reference))
  (bind _returnvalue (Transformation|GetActorLocation))
  (bind _outhits (Collision|MultiSphereTraceForObjects _returnvalue _returnvalue (Variables|Default|GetExplode%20Radius) (Variables|Default|GetExplode%20Trace%20Object%20Types) false (Utilities|Array|MakeArray [0] (Components|GetOwner)) "None" true "(R=1.000000,G=0.000000,B=0.000000,A=1.000000)" "(R=0.000000,G=1.000000,B=0.000000,A=1.000000)" 2.0))
  (for _array_element _outhits
    (if (and (< (Utilities|Array|FindItem (LocalVariables|GetDamagedActor) (.HitActor (Collision|BreakHitResult _array_element))) 0) (not (Class|AuraAbilitySystemLibrary|IsFriend (Components|GetOwner) (.HitActor (Collision|BreakHitResult _array_element)))))
      (Utilities|Array|AddUnique (LocalVariables|GetDamagedActor) (.HitActor (Collision|BreakHitResult _array_element)))
      (GameplayEffects|ApplyGameplayEffectSpecToSelf (Ability|GetAbilitySystemComponent (.HitActor (Collision|BreakHitResult _array_element))) (Variables|Default|GetDamageSpecHandle)))))