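; BP_FireVortexBolt is a fire projectile that follows a curving, returning path around its spawn point.
; A looping timer started on BeginPlay steadily reduces local forward speed into reverse while building sideways speed up to a cap.
; Each step also yaws the bolt along the line from its origin, so the local-space velocity bends into a swirl.
; The timer stops once forward speed has fully reversed, based on the launch speed.
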(event Custom|MoveTrack
  (bind _returnvalue (Transformation|GetActorLocation))
  (bind _origin_location (Variables|Default|GetOrigin%20Location))
  (bind _returnvalue_2 (- _returnvalue _origin_location))
  (bind _returnvalue_3 (Math|Rotator|MakeRotfromX _returnvalue_2))
  (Transformation|SetActorRotation (Math|Rotator|MakeRotator (.roll _returnvalue_3) 0.0 (.yaw _returnvalue_3)))
  (Variables|Default|SetLocalSpeedX (- (Variables|Default|GetLocalSpeedX) (Variables|Default|GetSpeedDelta)))
  (Variables|Default|SetLocalSpeedY (Math|Float|Clamp(Float) (+ (Variables|Default|GetLocalSpeedY) (Variables|Default|GetSpeedDelta)) 0.0 4.5e+02))
  (Game|Components|ProjectileMovement|SetVelocityinLocalSpace (Variables|Default|GetProjectileMovement) (Math|Vector|MakeVector (Variables|Default|GetLocalSpeedX) (Variables|Default|GetLocalSpeedY) 0.0))
  (bind _output_get (Variables|Default|SetTime (+ (Variables|Default|GetTime) (Variables|Default|GetSpeed%20Delta%20Time))))
  (if (>= _output_get (Variables|Default|GetReturn%20Time))
    (Utilities|Time|ClearandInvalidateTimerbyHandle (Variables|Default|GetTimer%20Handle))))

(event EventBeginPlay
  (Variables|Default|SetLocalSpeedX (Math|Vector|VectorLength (Transformation|GetVelocity)))
  (Variables|Default|SetOrigin%20Location (Transformation|GetActorLocation))
  (bind _returnvalue (Utilities|Time|SetTimerbyEvent (delegate Custom|MoveTrack) (Variables|Default|GetSpeed%20Delta%20Time) true))
  (Variables|Default|SetTimer%20Handle _returnvalue)
  (Variables|Default|SetReturn%20Time (* (Math|Float|SafeDivide (Variables|Default|GetLocalSpeedX) (Math|Float|SafeDivide (Variables|Default|GetSpeedDelta) (Variables|Default|GetSpeed%20Delta%20Time))) 2.0)))

(fn ConstructionScript
  (|CallParentFunction))