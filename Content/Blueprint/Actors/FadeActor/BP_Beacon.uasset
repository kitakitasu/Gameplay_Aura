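; Beacon actor that can fade its mesh out and back in through FadeOut and Fadein events.
; The construction script caches the original materials and builds dynamic instances from FadeMaterialInstance.
; FadeOut swaps in those instances and plays the FadeValue timeline, which drives their "Fade" parameter, while Fadein reverses it.
; When the timeline finishes at 1 or above, the original materials are restored and the fading flag clears.
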(event EventBeginPlay)

(event EventFadeOut
  (if (Variables|Default|GetIsFading)
    (bind _fadevalue (Timeline|FadeValue Play)
      (:Update
        (for _array_element (Variables|Default|GetDynamicMaterialInstance)
          (Rendering|Material|SetScalarParameterValue _array_element "Fade" _fadevalue :!class /Script/Engine.MaterialInstanceDynamic)))
      (:Finished
        (if (>= _fadevalue 1.0)
          (CallFunction|SetMeshMaterial false)
          (Variables|Default|SetIsFading false))))
    (else
      (Variables|Default|SetIsFading true)
      (CallFunction|SetMeshMaterial true)
      (Timeline|FadeValue PlayFromStart))))

(event EventFadein
  (bind _fadevalue (Timeline|FadeValue Reverse)
    (:Update
      (for _array_element (Variables|Default|GetDynamicMaterialInstance)
        (Rendering|Material|SetScalarParameterValue _array_element "Fade" _fadevalue :!class /Script/Engine.MaterialInstanceDynamic)))
    (:Finished
      (if (>= _fadevalue 1.0)
        (CallFunction|SetMeshMaterial false)
        (Variables|Default|SetIsFading false)))))

(fn ConstructionScript
  (Variables|Default|SetOriginalMaterials (Rendering|Material|GetMaterials (Variables|Default|GetMesh)))
  (for _array_element (Variables|Default|GetFadeMaterialInstance)
    (bind _returnvalue (Rendering|Material|CreateDynamicMaterialInstance _array_element "None" "None" :!class /Script/Engine.KismetMaterialLibrary))
    (Utilities|Array|AddUnique (Variables|Default|GetDynamicMaterialInstance) _returnvalue)))

(fn SetMeshMaterial
  (params (Dynamic? :type Boolean))
  (if Dynamic?
    (for (_array_element _array_index) (Variables|Default|GetDynamicMaterialInstance)
      (Rendering|Material|SetMaterial (Variables|Default|GetMesh) _array_index _array_element))
    (else
      (for (_array_element_2 _array_index_2) (Variables|Default|GetOriginalMaterials)
        (Rendering|Material|SetMaterial (Variables|Default|GetMesh) _array_index_2 _array_element_2)))))