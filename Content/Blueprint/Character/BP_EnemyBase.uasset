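; BP_EnemyBase is a base enemy character Blueprint handling startup attributes, death-style dissolve effects and attack facing.
; On BeginPlay it waits briefly, then initializes vital attributes.
; DissolveMesh creates dynamic material instances for the body and weapon meshes, with timelines driving their Dissolve parameter.
; SetFacingTargetLocation updates the FacingTarget motion warping target and draws a debug sphere at that location.
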(event EventBeginPlay
  (|CallParentFunction)
  ;[1 1 1 1 12] 忘记这是干什么了的的话看.h的注释，不要删
  (Utilities|FlowControl|Delay 0.2)
  (Class|AuraEnemy|InitializeVitalAttributes))

(event EventDissolveMesh
  (bind _dissolvemesh_mi (Variables|Default|GetDissolveMesh_MI))
  (bind _dissolveweaponmesh_mi (Variables|Default|GetDissolveWeaponMesh_MI))
  (Utilities|FlowControl|Sequence
    (:then_0
      (Utilities|IsValid _dissolvemesh_mi
        (:Is%20Valid
          (bind _returnvalue (Rendering|Material|CreateDynamicMaterialInstance _dissolvemesh_mi "Dissolve" "None" :!class /Script/Engine.KismetMaterialLibrary))
          (Rendering|Material|SetMaterial (Variables|Character|GetMesh) 0 _returnvalue)
          (bind _return_value (Timeline|Mesh%20Dissolve Play)
            (:Update
              (Rendering|Material|SetScalarParameterValue _returnvalue "Dissolve" _return_value :!class /Script/Engine.MaterialInstanceDynamic))))))
    (:then_1
      (Utilities|IsValid _dissolveweaponmesh_mi
        (:Is%20Valid
          (bind _returnvalue_2 (Rendering|Material|CreateDynamicMaterialInstance _dissolveweaponmesh_mi "Dissolve" "None" :!class /Script/Engine.KismetMaterialLibrary))
          (Rendering|Material|SetMaterial (Variables|Default|GetWeapon) 0 _returnvalue_2)
          (bind _return_value_2 (Timeline|Timeline Play)
            (:Update
              (Rendering|Material|SetScalarParameterValue _returnvalue_2 "Dissolve" _return_value_2 :!class /Script/Engine.MaterialInstanceDynamic))))))))

(event EventSetFacingTargetLocation
  (params (TargetLocation :type Vector%20%28by%20ref%29 :default "0, 0, 0"))
  (Rendering|Debug|DrawDebugSphere TargetLocation 5e+01 12 "(R=0.107419,G=1.000000,B=0.262970,A=1.000000)" 0.0)
  (Class|MotionWarpingComponent|AddorUpdateWarpTargetfromLocation (Variables|Default|GetMotionWarping) "FacingTarget" TargetLocation))

(fn ConstructionScript)