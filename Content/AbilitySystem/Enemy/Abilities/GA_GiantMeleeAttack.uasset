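; Gameplay ability for the Giant enemy's melee attack, which turns it toward its combat target and plays a random tagged attack montage.
; When the montage's gameplay event arrives, it sphere-traces at that attack's weapon socket.
; Each unique hit actor is damaged only if IsFriend returns true, which looks inverted given the function name.
; The ability ends when the montage completes, is interrupted or is cancelled.
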(event Ability|EventActivateAbility
  (bind _returnvalue (Ability|GetAvatarActorfromActorInfo))
  (bind _returnvalue_2 (Class|CombatInterface|GetCombatTarget(Message) _returnvalue))
  (Class|CombatInterface|SetFacingTargetLocation(Message) _returnvalue (Transformation|GetActorLocation _returnvalue_2))
  (bind _returnvalue_3 (Class|CombatInterface|GetAttackMontages(Message) (Ability|GetAvatarActorfromActorInfo)))
  (bind _output_get (Variables|Default|SetTaggedMontage (.OutItem (Utilities|Array|Random _returnvalue_3))))
  (|PlayMontageandWaitProxy "None" (.Montage (Utilities|Struct|BreakTaggedMontage _output_get)) 1.0 "None" true 1.0 0.0 false
    (:then
      (Ability|Tasks|WaitGameplayEvent (.MontageTag (Utilities|Struct|BreakTaggedMontage _output_get)) 0
        (:EventReceived
          (bind _returnvalue_4 (Class|CombatInterface|GetWeaponSocketLocation(Message) (Ability|GetAvatarActorfromActorInfo) (.MontageTag (Utilities|Struct|BreakTaggedMontage _output_get))))
          (bind _outhits (Collision|MultiSphereTraceByChannel _returnvalue_4 _returnvalue_4 6e+01 "TraceTypeQuery1" false 0 "None"))
          (bind _array_element (Utilities|Array|ForEachLoopwithBreak _outhits)
            (:LoopBody
              (if (== (Utilities|Array|FindItem (Variables|Default|GetOverlapActors) (.HitActor (Collision|BreakHitResult _array_element))) -1)
                (Utilities|Array|Add (Variables|Default|GetOverlapActors) (.HitActor (Collision|BreakHitResult _array_element)))
                (if (Class|AuraAbilitySystemLibrary|IsFriend (.HitActor (Collision|BreakHitResult _array_element)) (Ability|GetAvatarActorfromActorInfo))
                  (Class|AuraDamageGameplayAbility|CauseDamage (.HitActor (Collision|BreakHitResult _array_element))))))
            (:Completed
              (Utilities|Array|Clear (Variables|Default|GetOverlapActors)))))))
    (:OnCompleted
      (Ability|EndAbility :!label _label))
    (:OnInterrupted
      (goto _label))
    (:OnCancelled
      (goto _label))))