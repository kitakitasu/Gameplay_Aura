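; GA_EnemyHitReact is the gameplay ability that plays an enemy's hit reaction.
; On activation it applies the GE_HitReact effect to itself, stores the handle, and plays the montage the avatar supplies through CombatInterface.
; When the montage completes, is interrupted or is cancelled, it removes that effect by handle and ends the ability.
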(event Ability|EventActivateAbility
  (bind _returnvalue (Ability|GetAvatarActorfromActorInfo))
  (bind _returnvalue_2 (Ability|GetAbilitySystemComponent _returnvalue))
  (bind _returnvalue_3 (Ability|ApplyGameplayEffectSpecToOwner (GameplayEffects|MakeOutgoingSpec _returnvalue_2 "/Game/AbilitySystem/Enemy/GameplayEffects/GE_HitReact.GE_HitReact_C" 1.0 (GameplayEffects|MakeEffectContext _returnvalue_2))))
  (Variables|Default|SetHit%20React%20Effect%20Handle _returnvalue_3)
  (bind _ascombat_interface (Utilities|Casting|CastToCombatInterface (Ability|GetAvatarActorfromActorInfo)))
  (bind _returnvalue_4 (Class|CombatInterface|GetHitReactMontage _ascombat_interface))
  (|PlayMontageandWaitProxy "None" _returnvalue_4 1.0 "None" true 1.0 0.0 false
    (:OnCompleted
      _)
    (:OnInterrupted
      _)
    (:OnCancelled
      _))
  (Ability|RemoveGameplayEffectFromOwnerWithHandle (Variables|Default|GetHit%20React%20Effect%20Handle))
  (Ability|EndAbility))

(event Ability|EventOnEndAbility
  (params (bWasCancelled :type Boolean)))