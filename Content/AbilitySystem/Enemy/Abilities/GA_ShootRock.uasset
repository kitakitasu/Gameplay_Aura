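; GA_ShootRock is an enemy gameplay ability that fires a rock projectile at the combat target.
; On activation it faces the avatar toward the target's location and plays the first attack montage from the avatar's interface messages.
; A gameplay event matching that montage's tag spawns the projectile toward the location captured at activation.
; The ability ends when the montage completes, is interrupted or is cancelled.
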(event Ability|EventActivateAbility
  (bind _returnvalue (Ability|GetAvatarActorfromActorInfo))
  (bind _returnvalue_2 (Class|CombatInterface|GetCombatTarget(Message) _returnvalue))
  (bind _output_get (Variables|Default|SetTargetLocation (Transformation|GetActorLocation _returnvalue_2)))
  (Class|CombatInterface|SetFacingTargetLocation(Message) _returnvalue _output_get)
  (bind _returnvalue_3 (Class|CombatInterface|GetAttackMontages(Message) (Ability|GetAvatarActorfromActorInfo)))
  (|PlayMontageandWaitProxy "None" (.montage (Utilities|Array|Get(acopy) _returnvalue_3)) 1.0 "None" true 1.0 0.0 false
    (:then
      (Ability|Tasks|WaitGameplayEvent (.montagetag (Utilities|Array|Get(acopy) _returnvalue_3)) 0
        (:EventReceived
          (Class|AuraProjectileSpell|SpawnProjectile (Variables|Default|GetTargetLocation)))))
    (:OnCompleted
      (Ability|EndAbility :!label _label))
    (:OnInterrupted
      (goto _label))
    (:OnCancelled
      (goto _label))))