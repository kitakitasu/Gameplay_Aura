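; Enemy melee attack gameplay ability that faces the combat target and plays a random tagged attack montage.
; A gameplay event matching the montage's tag triggers a sphere trace at that montage's weapon socket.
; Each unique non-friendly actor hit takes damage and fires a melee impact gameplay cue carrying the montage tag.
; The ability ends when the montage completes, is interrupted or is cancelled.
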(event Ability|EventActivateAbility
  (bind _returnvalue (Ability|GetAvatarActorfromActorInfo))
  (bind _returnvalue_2 (Class|CombatInterface|GetCombatTarget(Message) _returnvalue))
  (Class|CombatInterface|SetFacingTargetLocation(Message) _returnvalue (Transformation|GetActorLocation _returnvalue_2))
  (bind _returnvalue_3 (Class|CombatInterface|GetAttackMontages(Message) (Ability|GetAvatarActorfromActorInfo)))
  (bind _output_get (Variables|Default|SetTaggedMontage (.OutItem (Utilities|Array|Random _returnvalue_3))))
  (|PlayMontageandWaitProxy "None" (.Montage (Utilities|Struct|BreakTaggedMontage _output_get)) 1.0 "None" true 1.0 0.0 false
    (:then
      (Ability|Tasks|WaitGameplayEvent (.MontageTag (Utilities|Struct|BreakTaggedMontage _output_get)) 0
        (:EventReceived
          (bind _returnvalue_4 (Class|CombatInterface|GetWeaponSocketLocation(Message) (Ability|GetAvatarActorfromActorInfo) (.CombatSocketTag (Utilities|Struct|BreakTaggedMontage _output_get))))
          (bind _output_get_2 (Variables|Default|SetWeaponSocketLocation _returnvalue_4))
          (bind _outhits (Collision|MultiSphereTraceByChannel _output_get_2 _output_get_2 45.0 "TraceTypeQuery1" false 0 "None"))
          (bind _array_element (Utilities|Array|ForEachLoopwithBreak _outhits)
            (:LoopBody
              (if (== (Utilities|Array|FindItem (Variables|Default|GetOverlapActors) (.HitActor (Collision|BreakHitResult _array_element))) -1)
                (Utilities|Array|Add (Variables|Default|GetOverlapActors) (.HitActor (Collision|BreakHitResult _array_element)))
                (if (not (Class|AuraAbilitySystemLibrary|IsFriend (.HitActor (Collision|BreakHitResult _array_element)) (Ability|GetAvatarActorfromActorInfo)))
                  (Class|AuraDamageGameplayAbility|CauseDamage (.HitActor (Collision|BreakHitResult _array_element)))
                  (Class|GameplayAbility|ExecuteGameplayCuewithParams "(TagName=\"GameplayCue.MeleeImpact\")" (Ability|GameplayCue|MakeGameplayCueParameters :AggregatedSourceTags (GameplayTags|MakeGameplayTagContainerfromTag (.montagetag (Variables|Default|GetTaggedMontage))) :Location (Variables|Default|GetWeaponSocketLocation) :EffectCauser (Ability|GetAvatarActorfromActorInfo) :SourceObject (.HitActor (Collision|BreakHitResult _array_element)))))))
            (:Completed
              (Utilities|Array|Clear (Variables|Default|GetOverlapActors)))))))
    (:OnCompleted
      (Ability|EndAbility :!label _label))
    (:OnInterrupted
      (goto _label))
    (:OnCancelled
      (goto _label))))