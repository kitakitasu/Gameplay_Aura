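; Enemy gameplay ability that has the Shaman summon random minions, up to the number it can still call.
; It faces the combat target, plays the summon montage, then on a montage gameplay event shuffles the spawn locations and starts a looping timer.
; Each tick spawns a Niagara effect and a minion with controller and owner, and increments the avatar's minion count.
; When none remain callable, it ends and clears the timer.
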(event Custom|SpawnMinions
  (bind _returnvalue (Class|CombatInterface|GetCallableMinionNum(Message) (Ability|GetAvatarActorfromActorInfo)))
  (Variables|Default|SetIndex _returnvalue)
  (if (> _returnvalue 0)
    (Niagara|SpawnSystematLocation "/Game/Assets/Effects/Combat/NS_GroundSummon.NS_GroundSummon" (Utilities|Array|Get(acopy) (Variables|Default|GetSpawnLocations) (Variables|Default|GetIndex)))
    (bind _returnvalue_2 (Game|SpawnActorfromClass (Class|SummonAbility|GetRandomMinionClass) (Math|Transform|MakeTransform (+ (Utilities|Array|Get(acopy) (Variables|Default|GetSpawnLocations) (Variables|Default|GetIndex)) "0.000000,0.000000,80.000000") (Transformation|GetActorRotation (Ability|GetAvatarActorfromActorInfo)) "1.000000,1.000000,1.000000") "AdjustIfPossibleButDontSpawnIfColliding" "MultiplyWithRoot" 0 0))
    (Utilities|IsValid _returnvalue_2
      (:Is%20Valid
        (Pawn|SpawnDefaultController _returnvalue_2)
        (Actor|SetOwner _returnvalue_2 (Ability|GetAvatarActorfromActorInfo)))
      (:Is%20Not%20Valid
        _))
    (Class|CombatInterface|IncreaseMinionNum(Message) (Ability|GetAvatarActorfromActorInfo) 1)
    (else
      (Ability|EndAbility)
      (Utilities|Time|ClearandInvalidateTimerbyHandle (Variables|Default|GetSpawnTimer)))))

(event Ability|EventActivateAbility
  (bind _returnvalue (Ability|GetAvatarActorfromActorInfo))
  (bind _returnvalue_2 (Class|CombatInterface|GetCallableMinionNum(Message) (Ability|GetAvatarActorfromActorInfo)))
  (Variables|Default|SetNumMinions _returnvalue_2)
  (bind _returnvalue_3 (Class|CombatInterface|GetCombatTarget(Message) _returnvalue))
  (Class|CombatInterface|SetFacingTargetLocation(Message) _returnvalue (Transformation|GetActorLocation _returnvalue_3))
  (|PlayMontageandWaitProxy "None" "/Game/Assets/Enemies/Shaman/Animations/AM_Shaman_Summon.AM_Shaman_Summon" 1.0 "None" true 1.0 0.0 false
    (:then
      (Ability|Tasks|WaitGameplayEvent "(TagName=\"Montage.Attack.2\")" 0 true
        (:EventReceived
          (bind _returnvalue_4 (Class|SummonAbility|GetSpawnLocation))
          (bind _output_get (Variables|Default|SetSpawnLocations _returnvalue_4))
          (Utilities|Array|Shuffle _output_get)
          (bind _returnvalue_5 (Utilities|Time|SetTimerbyEvent (delegate Custom|SpawnMinions) 0.2 true))
          (Variables|Default|SetSpawnTimer _returnvalue_5))))))