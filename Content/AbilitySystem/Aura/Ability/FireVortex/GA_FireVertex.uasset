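; Fire Vortex gameplay ability for Aura that fires eight projectiles in a ring outward from the caster.
; After committing, it gets target data under the mouse, turns the caster toward it and plays the Arcane Shards cast montage.
; The Event.Montage.FireVortex event triggers the spawns, with start and target points computed at 45-degree yaw steps around the avatar.
; The ability ends when the montage completes, blends out, is interrupted or cancelled.
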(event Ability|EventActivateAbility
  (bind _returnvalue (Ability|CommitAbility))
  (if _returnvalue
    (bind _data (|TargetDataUnderMouse)
      (:ValidData
        (bind _ascombat_interface (Utilities|Casting|CastToCombatInterface (Ability|GetAvatarActorfromActorInfo)))
        (Class|CombatInterface|SetFacingTargetLocation _ascombat_interface (.Location (Collision|BreakHitResult (Ability|TargetData|GetHitResultfromTargetData _data))))
        (|PlayMontageandWaitProxy "None" "/Game/Assets/Characters/Cleric_VRoid/Animation/AM_Cast_ArcaneShards.AM_Cast_ArcaneShards" 1.0 "None" false 1.0 0.0 false
          (:then
            (Ability|Tasks|WaitGameplayEvent "(TagName=\"Event.Montage.FireVortex\")" 0
              (:EventReceived
                (for _index (range 1 8)
                  (Class|AuraProjectileSpell|SpawnProjectile (.TargetLocation (CallFunction|CalculateProjectileRotationLocation _index)) (GameplayTags|MakeLiteralGameplayTag "(TagName=\"CombatSocket.Weapon\")") (.SpawnLocation (CallFunction|CalculateProjectileRotationLocation _index)))))))
          (:OnCompleted
            (Ability|EndAbility :!label _label))
          (:OnBlendOut
            (goto _label))
          (:OnInterrupted
            (goto _label))
          (:OnCancelled
            (goto _label)))))))

(fn CalculateProjectileRotationLocation
  (params (Num :type Integer))
  (bind _returnvalue (Ability|GetAvatarActorfromActorInfo))
  (bind _returnvalue_2 (* Num 45.0))
  (bind _returnvalue_3 (Transformation|GetActorRotation _returnvalue))
  (bind _returnvalue_4 (Transformation|GetActorLocation _returnvalue))
  (bind _returnvalue_5 (+ _returnvalue_2 (.yaw _returnvalue_3)))
  (bind _returnvalue_6 (Math|Rotator|GetRotationXVector (Math|Rotator|MakeRotator (.roll _returnvalue_3) (.pitch _returnvalue_3) _returnvalue_5)))
  (return (+ _returnvalue_4 (* _returnvalue_6 3e+02)) (+ _returnvalue_4 (* _returnvalue_6 5e+01))))