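; GA_ArcaneBolt is a gameplay ability that fires a projectile from the weapon socket toward the target under the mouse.
; After committing, it gets mouse target data, turns the caster toward the hit location and plays the FireBolt cast montage.
; The montage's FireBolt gameplay event triggers the projectile spawn, and the ability ends when the montage completes, blends out, is interrupted or is cancelled.
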(event Ability|EventActivateAbility
  (bind _returnvalue (Ability|CommitAbility))
  (if _returnvalue
    (bind _data (|TargetDataUnderMouse)
      (:ValidData
        (bind _ascombat_interface (Utilities|Casting|CastToCombatInterface (Ability|GetAvatarActorfromActorInfo)))
        (Class|CombatInterface|SetFacingTargetLocation _ascombat_interface (.Location (Collision|BreakHitResult (Ability|TargetData|GetHitResultfromTargetData _data))))
        (|PlayMontageandWaitProxy "None" "/Game/Assets/Characters/Cleric_VRoid/Animation/AM_Cast_FireBolt.AM_Cast_FireBolt" 1.0 "None" false 1.0 0.0 false
          (:then
            (Ability|Tasks|WaitGameplayEvent "(TagName=\"Event.Montage.FIreBolt\")" 0
              (:EventReceived
                (Class|AuraProjectileSpell|SpawnProjectile (.Location (Collision|BreakHitResult (Ability|TargetData|GetHitResultfromTargetData _data))) (GameplayTags|MakeLiteralGameplayTag "(TagName=\"CombatSocket.Weapon\")")))))
          (:OnCompleted
            (Ability|EndAbility :!label _label))
          (:OnBlendOut
            (goto _label))
          (:OnInterrupted
            (goto _label))
          (:OnCancelled
            (goto _label)))))))